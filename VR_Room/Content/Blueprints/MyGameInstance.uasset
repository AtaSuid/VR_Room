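; Game instance that handles multiplayer session hosting, searching and joining through Advanced Sessions nodes.
; CreateSession creates a session and, on success, opens the Small_2-4 map as a listen server.
; FindSession stores the search results, loops through them with an empty body, then joins using the loop's last element.
; The separate Join event joins a supplied session and prints a message on failure.
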(event Custom|Join
  (params (Session%20to%20Join :type Blueprint%20Session%20Result%20Structure))
  (|JoinSession (Game|GetPlayerController 0) Session%20to%20Join
    (:OnFailure
      (Development|PrintString "failed"))))

(event Custom|Create%20Session
  (|AdvancedSession 0 (Game|GetPlayerController 0) 100 0 false true false true true false false false true
    (:OnSuccess
      (Game|OpenLevel(byName) "Small_2-4" true "listen"))))

(event Custom|FindSession
  (bind _results (|FindSessionsAdvanced (Game|GetPlayerController 0) 10 false "AllServers" 0 false false false)
    (:OnSuccess
      (bind _output_get (Variables|Default|SetFoundSession _results))
      (for _array_element _output_get
        _)
      (|JoinSession (Game|GetPlayerController 0) _array_element))))